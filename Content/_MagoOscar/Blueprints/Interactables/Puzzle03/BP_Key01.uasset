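; BP_Key01 is an interactable for Puzzle03 that acts as one cycling digit from 0 to 9.
; On interact it finds BP_Puzzle03, increments that actor's Key01 value and wraps it to 0 after 9.
; It writes the new value to the W_Num widget on its Widget component, then calls the puzzle's Check.
; The puzzle actor holds the digit, and the key prints a debug string on each interaction.
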(event EventOnInteract
  (Development|PrintString "Descripción")
  (bind _returnvalue (Actor|GetActorOfClass "/Game/_MagoOscar/Blueprints/Interactables/Puzzle03/BP_Puzzle03.BP_Puzzle03_C"))
  (bind _output_get (Variables|/Game/_MagoOscar/Blueprints/Interactables/Puzzle03/BP_Puzzle03.BP_Puzzle03_C|SetKey01 _returnvalue (+ (Variables|/Game/_MagoOscar/Blueprints/Interactables/Puzzle03/BP_Puzzle03.BP_Puzzle03_C|GetKey01 _returnvalue) 1)))
  (if (> _output_get 9)
    (bind _output_get_2 (Variables|/Game/_MagoOscar/Blueprints/Interactables/Puzzle03/BP_Puzzle03.BP_Puzzle03_C|SetKey01 _returnvalue 0))
    (bind _asw_num (Utilities|Casting|CastToW_Num (UserInterface|GetUserWidgetObject (Variables|Default|GetWidget))))
    (Variables|/Game/_MagoOscar/Widgets/W_Num.W_Num_C|SetValue _asw_num _output_get_2)
    (else
      (bind _asw_num_2 (Utilities|Casting|CastToW_Num (UserInterface|GetUserWidgetObject (Variables|Default|GetWidget))))
      (Variables|/Game/_MagoOscar/Widgets/W_Num.W_Num_C|SetValue _asw_num_2 _output_get)))
  (Default|Check _returnvalue))

(fn ConstructionScript
  (|CallParentFunction))