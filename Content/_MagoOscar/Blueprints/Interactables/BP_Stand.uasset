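; BP_Stand is an interactable pedestal that takes the player's three key gems and summons the final boss.
; On interact it reads the red, blue and green key flags from CH_PlayerCharacter and shows the matching gem components.
; With all three, it moves BP_FinalBoss to its Arrow, starts it following the player, switches the music and destroys itself.
; Otherwise it shows a timed sequence of indication messages on the player UI.
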(event EventOnInteract
  (|CallParentFunction)
  (bind _asch_player_character (Utilities|Casting|CastToCH_PlayerCharacter (Game|GetPlayerCharacter 0)))
  (Utilities|FlowControl|Sequence
    (:then_0
      (bind _output_get (Variables|Default|SetRedGem (Variables|/Game/_MagoOscar/Blueprints/Player/CH_PlayerCharacter.CH_PlayerCharacter_C|GetRedKey _asch_player_character)))
      (if _output_get
        (Rendering|SetVisibility (Variables|Default|GetRed) true false)))
    (:then_1
      (bind _output_get_2 (Variables|Default|SetBlueGem (Variables|/Game/_MagoOscar/Blueprints/Player/CH_PlayerCharacter.CH_PlayerCharacter_C|GetBlueKey _asch_player_character)))
      (if _output_get_2
        (Rendering|SetVisibility (Variables|Default|GetBlue) true false)))
    (:then_2
      (bind _output_get_3 (Variables|Default|SetGreenGem (Variables|/Game/_MagoOscar/Blueprints/Player/CH_PlayerCharacter.CH_PlayerCharacter_C|GetGreenKey _asch_player_character)))
      (if _output_get_3
        (Rendering|SetVisibility (Variables|Default|GetGreen) true false)))
    (:then_3
      (if (Variables|Default|GetRedGem)
        (if (Variables|Default|GetGreenGem)
          (if (Variables|Default|GetBlueGem)
            (bind _returnvalue (Actor|GetActorOfClass "/Game/_MagoOscar/Blueprints/Enemies/BP_FinalBoss.BP_FinalBoss_C"))
            (Transformation|SetActorLocation _returnvalue (Transformation|GetWorldLocation (Variables|Default|GetArrow)) false false)
            (Default|FollowPlayer _returnvalue)
            (bind _returnvalue_2 (Actor|GetActorOfClass "/Game/_MagoOscar/Audio/BP_MusicManager.BP_MusicManager_C"))
            (Default|PlayMusic _returnvalue_2 "/Game/_MagoOscar/Audio/Protection_of_Kingdom__looped_.Protection_of_Kingdom__looped_" 0.0)
            (Actor|DestroyActor)
            (else
              (Variables|/Game/_MagoOscar/Blueprints/Player/WB_PlayerUI.WB_PlayerUI_C|SetContent (Variables|/Game/_MagoOscar/Blueprints/Player/CH_PlayerCharacter.CH_PlayerCharacter_C|GetPlayerUI _asch_player_character) (Variables|Default|GetIndication) :!label _label)
              (Utilities|FlowControl|Delay 2.0)
              (Variables|/Game/_MagoOscar/Blueprints/Player/WB_PlayerUI.WB_PlayerUI_C|SetContent (Variables|/Game/_MagoOscar/Blueprints/Player/CH_PlayerCharacter.CH_PlayerCharacter_C|GetPlayerUI _asch_player_character) (Variables|Default|GetIndication01))
              (Utilities|FlowControl|Delay 2.0)
              (Variables|/Game/_MagoOscar/Blueprints/Player/WB_PlayerUI.WB_PlayerUI_C|SetContent (Variables|/Game/_MagoOscar/Blueprints/Player/CH_PlayerCharacter.CH_PlayerCharacter_C|GetPlayerUI _asch_player_character) (Variables|Default|GetIndication02))
              (Utilities|FlowControl|Delay 2.0)
              (Variables|/Game/_MagoOscar/Blueprints/Player/WB_PlayerUI.WB_PlayerUI_C|SetContent (Variables|/Game/_MagoOscar/Blueprints/Player/CH_PlayerCharacter.CH_PlayerCharacter_C|GetPlayerUI _asch_player_character) (Variables|Default|GetIndication03))
              (Utilities|FlowControl|Delay 2.0)
              (Variables|/Game/_MagoOscar/Blueprints/Player/WB_PlayerUI.WB_PlayerUI_C|SetContent (Variables|/Game/_MagoOscar/Blueprints/Player/CH_PlayerCharacter.CH_PlayerCharacter_C|GetPlayerUI _asch_player_character) "")))
          (else
            (goto _label)))
        (else
          (goto _label))))))

(fn ConstructionScript
  (|CallParentFunction))