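; Final boss enemy character that chases the player, attacks with a greatsword, and plays a victory dance once the player is dying.
; An AI MoveTo loop closes in and triggers the attack; sword overlaps deal damage only while attacking.
; Incoming damage updates the life bar widget and either staggers the boss before it resumes chasing or kills and later destroys it.
; Actions play as single animations, then restore the Animation Blueprint.
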(event OnComponentBeginOverlap(SM_Wep_Greatsword_Round_01)
  (params (OverlappedComponent :type Primitive%20Component%20Object%20Reference) (OtherActor :type Actor%20Object%20Reference) (OtherComp :type Primitive%20Component%20Object%20Reference) (OtherBodyIndex :type Integer) (bFromSweep :type Boolean) (SweepResult :type Hit%20Result%20Structure%20%28by%20ref%29))
  (if (Variables|Default|GetIsAttacking)
    (Game|Damage|ApplyDamage OtherActor 2.0 0 0)))

(event Custom|FollowPlayer
  (bind _returnvalue (Game|GetPlayerCharacter 0))
  (if (not (Variables|Default|GetIsDamaged))
    (if (not (Variables|Default|GetIsDying))
      (if (not (Variables|Default|GetIsAttacking))
        (AI|AIMoveTo self "0, 0, 0" _returnvalue 2e+02 false
          (:OnSuccess
            (if (not (Variables|Default|GetIsDying))
              (CallFunction|Attack)
              (Utilities|FlowControl|Delay 1.0)
              (Variables|Default|SetIsAttacking false)
              (Utilities|FlowControl|Delay 0.5)
              (bind _asch_player_character (Utilities|Casting|CastToCH_PlayerCharacter _returnvalue))
              (if (Variables|/Game/_MagoOscar/Blueprints/Player/CH_PlayerCharacter.CH_PlayerCharacter_C|GetIsDying _asch_player_character)
                (Components|Animation|PlayAnimation (Variables|Character|GetMesh) "/Game/_MagoOscar/Animation/Animation/BossAnim/VictoryDance.VictoryDance" false)
                (else
                  (Components|Animation|SetAnimationMode (Variables|Character|GetMesh) "AnimationBlueprint" true)
                  (Variables|/Script/Engine.CharacterMovementComponent|SetMaxWalkSpeed (Variables|Character|GetCharacterMovement) 3e+02)
                  (CallFunction|FollowPlayer)))))
          (:OnFail
            (CallFunction|FollowPlayer)))))))

(event Custom|TakeDamage
  (params (Damage :type Float%20%28double-precision%29))
  (Rendering|SetVisibility (Variables|Default|GetWidget) true false)
  (if (not (Variables|Default|GetIsDying))
    (bind _output_get (Variables|Default|SetHealth (- (Variables|Default|GetHealth) Damage)))
    (bind _asw_boss_life_bar (Utilities|Casting|CastToW_BossLifeBar (UserInterface|GetUserWidgetObject (Variables|Default|GetWidget))))
    (Variables|/Game/_MagoOscar/Widgets/W_BossLifeBar.W_BossLifeBar_C|SetHealth _asw_boss_life_bar _output_get)
    (if (<= _output_get 0.0)
      (CallFunction|Death)
      (Utilities|FlowControl|Delay 1e+01)
      (Actor|DestroyActor)
      (else
        (CallFunction|RecibeDamage)
        (Utilities|FlowControl|Delay 0.7)
        (Components|Animation|SetAnimationMode (Variables|Character|GetMesh) "AnimationBlueprint" true)
        (Variables|Default|SetIsDamaged false)
        (Variables|/Script/Engine.CharacterMovementComponent|SetMaxWalkSpeed (Variables|Character|GetCharacterMovement) 3e+02)
        (CallFunction|FollowPlayer)))))

(event EventBeginPlay
  (CallFunction|FollowPlayer))

(event Game|Damage|EventAnyDamage
  (params (Damage :type Float%20%28single-precision%29) (DamageType :type Damage%20Type%20Object%20Reference) (InstigatedBy :type Controller%20Object%20Reference) (DamageCauser :type Actor%20Object%20Reference))
  (Development|PrintString (Utilities|GetDisplayName DamageCauser))
  (if (!= DamageCauser self)
    (CallFunction|TakeDamage Damage)))

(fn ConstructionScript)

(fn Attack
  (Variables|Default|SetIsAttacking true)
  (Components|Animation|PlayAnimation (Variables|Character|GetMesh) "/Game/_MagoOscar/Animation/Animation/BossAnim/Sword.Sword" false))

(fn Death
  (Variables|Default|SetIsDying true)
  (Components|Animation|PlayAnimation (Variables|Character|GetMesh) "/Game/_MagoOscar/Animation/Animation/BossAnim/Death.Death" false)
  (Variables|/Script/Engine.CharacterMovementComponent|SetMaxWalkSpeed (Variables|Character|GetCharacterMovement) 0.0))

(fn RecibeDamage
  (Variables|Default|SetIsDamaged true)
  (Components|Animation|PlayAnimation (Variables|Character|GetMesh) "/Game/_MagoOscar/Animation/Animation/BossAnim/impact.impact" false)
  (Variables|/Script/Engine.CharacterMovementComponent|SetMaxWalkSpeed (Variables|Character|GetCharacterMovement) 0.0))