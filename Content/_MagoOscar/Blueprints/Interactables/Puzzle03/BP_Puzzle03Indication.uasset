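; BP_Puzzle03Indication is an interactable that shows timed indication text for Puzzle 03 on the player's UI.
; On interact, it casts the player character to CH_PlayerCharacter and writes three indication variables in sequence to that character's PlayerUI content.
; Fixed delays hold each message on screen, and the content is cleared after the last one.
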(event EventOnInteract
  (bind _asch_player_character (Utilities|Casting|CastToCH_PlayerCharacter (Game|GetPlayerCharacter 0)))
  (Variables|/Game/_MagoOscar/Blueprints/Player/WB_PlayerUI.WB_PlayerUI_C|SetContent (Variables|/Game/_MagoOscar/Blueprints/Player/CH_PlayerCharacter.CH_PlayerCharacter_C|GetPlayerUI _asch_player_character) (Variables|Default|GetIndication))
  (Utilities|FlowControl|Delay 4.0)
  (Variables|/Game/_MagoOscar/Blueprints/Player/WB_PlayerUI.WB_PlayerUI_C|SetContent (Variables|/Game/_MagoOscar/Blueprints/Player/CH_PlayerCharacter.CH_PlayerCharacter_C|GetPlayerUI _asch_player_character) (Variables|Default|GetIndication01))
  (Utilities|FlowControl|Delay 4.0)
  (Variables|/Game/_MagoOscar/Blueprints/Player/WB_PlayerUI.WB_PlayerUI_C|SetContent (Variables|/Game/_MagoOscar/Blueprints/Player/CH_PlayerCharacter.CH_PlayerCharacter_C|GetPlayerUI _asch_player_character) (Variables|Default|GetIndication02))
  (Utilities|FlowControl|Delay 4.0)
  (Variables|/Game/_MagoOscar/Blueprints/Player/WB_PlayerUI.WB_PlayerUI_C|SetContent (Variables|/Game/_MagoOscar/Blueprints/Player/CH_PlayerCharacter.CH_PlayerCharacter_C|GetPlayerUI _asch_player_character) ""))

(fn ConstructionScript
  (|CallParentFunction))