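; BP_Key is an interactable key pickup that adds one key to the player's count.
; On interact, it runs the parent logic, increments Keys on CH_PlayerCharacter and copies the total to the player's UI.
; It then plays a coin sound through the BP_MusicManager found in the level and destroys itself.
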(event EventOnInteract
  (|CallParentFunction)
  (bind _asch_player_character (Utilities|Casting|CastToCH_PlayerCharacter (Game|GetPlayerCharacter 0)))
  (bind _output_get (Variables|/Game/_MagoOscar/Blueprints/Player/CH_PlayerCharacter.CH_PlayerCharacter_C|SetKeys _asch_player_character (+ (Variables|/Game/_MagoOscar/Blueprints/Player/CH_PlayerCharacter.CH_PlayerCharacter_C|GetKeys _asch_player_character) 1)))
  (Variables|/Game/_MagoOscar/Blueprints/Player/WB_PlayerUI.WB_PlayerUI_C|SetKeys (Variables|/Game/_MagoOscar/Blueprints/Player/CH_PlayerCharacter.CH_PlayerCharacter_C|GetPlayerUI _asch_player_character) _output_get)
  (bind _returnvalue (Actor|GetActorOfClass "/Game/_MagoOscar/Audio/BP_MusicManager.BP_MusicManager_C"))
  (Default|PlayFX _returnvalue "/Game/_MagoOscar/Audio/Coins_19.Coins_19")
  (Actor|DestroyActor))

(fn ConstructionScript
  (|CallParentFunction))