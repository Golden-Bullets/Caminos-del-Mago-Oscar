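; BP_TestEnemy is a simple test enemy that wanders the navmesh and can be damaged and killed.
; MoveAround picks a random navigable point near the actor, moves there with AI MoveTo, then waits and calls itself again on success.
; AnyDamage forwards to TakeDamage, which lowers Health, prints it, and calls Death to destroy the actor at zero or below.
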(event Custom|TakeDamage
  (params (Damage :type Float%20%28double-precision%29))
  (bind _output_get (Variables|Default|SetHealth (- (Variables|Default|GetHealth) Damage)))
  (Development|PrintString (Utilities|String|ToString(Float) _output_get))
  (if (<= _output_get 0.0)
    (CallFunction|Death)))

(event Custom|MoveAround
  (bind _randomlocation (Class|NavigationSystemV1|GetRandomLocationinNavigableRadius (Transformation|GetActorLocation) 1e+03 0 0))
  (AI|AIMoveTo 0 _randomlocation 0 5.0 false
    (:OnSuccess
      (Utilities|FlowControl|Delay 3.0)
      (CallFunction|MoveAround))))

(event Game|Damage|EventAnyDamage
  (params (Damage :type Float%20%28single-precision%29) (DamageType :type Damage%20Type%20Object%20Reference) (InstigatedBy :type Controller%20Object%20Reference) (DamageCauser :type Actor%20Object%20Reference))
  (CallFunction|TakeDamage Damage))

(fn ConstructionScript)

(fn Death
  (Actor|DestroyActor))