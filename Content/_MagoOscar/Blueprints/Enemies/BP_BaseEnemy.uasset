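; Base melee enemy character that wanders the navmesh, chases pawns it sees and attacks with a club.
; PawnSensing or surviving a hit triggers the chase; after an attack it slows and resumes wandering.
; Club overlaps deal damage only while attacking, and incoming damage updates a life-bar widget, ending in death and destruction.
; Boolean flags gate states, while attack, hit and death animations play directly on the mesh, overriding the AnimBP.
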(event OnSeePawn(PawnSensing)
  (params (Pawn :type Pawn%20Object%20Reference))
  (CallFunction|FollowPlayer Pawn))

(event OnComponentBeginOverlap(SM_Wep_Goblin_Club_01)
  (params (OverlappedComponent :type Primitive%20Component%20Object%20Reference) (OtherActor :type Actor%20Object%20Reference) (OtherComp :type Primitive%20Component%20Object%20Reference) (OtherBodyIndex :type Integer) (bFromSweep :type Boolean) (SweepResult :type Hit%20Result%20Structure%20%28by%20ref%29))
  (if (Variables|Default|GetIsAttacking)
    (Game|Damage|ApplyDamage OtherActor 1.0 0 0)))

(event Custom|FollowPlayer
  (params (Pawn :type Pawn%20Object%20Reference))
  (if (not (Variables|Default|GetIsDamaged))
    (if (not (Variables|Default|GetIsDying))
      (if (not (Variables|Default|GetIsAttacking))
        (Utilities|FlowControl|Sequence
          (:then_0
            (Variables|/Script/Engine.CharacterMovementComponent|SetMaxWalkSpeed (Variables|Character|GetCharacterMovement) 3e+02))
          (:then_1
            (AI|AIMoveTo self "0, 0, 0" Pawn 2e+02 false
              (:OnSuccess
                (if (not (Variables|Default|GetIsDying))
                  (CallFunction|Attack)
                  (Utilities|FlowControl|Delay 1.0)
                  (Variables|Default|SetIsAttacking false)
                  (Utilities|FlowControl|Delay 0.5)
                  (Components|Animation|SetAnimationMode (Variables|Character|GetMesh) "AnimationBlueprint" true)
                  (Variables|/Script/Engine.CharacterMovementComponent|SetMaxWalkSpeed (Variables|Character|GetCharacterMovement) 1.3e+02)
                  (CallFunction|MoveAround))))))))))

(event Custom|TakeDamage
  (params (Damage :type Float%20%28double-precision%29))
  (Rendering|SetVisibility (Variables|Default|GetWidget) true false)
  (if (not (Variables|Default|GetIsDying))
    (bind _output_get (Variables|Default|SetHealth (- (Variables|Default|GetHealth) Damage)))
    (bind _asw_enemy_life_bar (Utilities|Casting|CastToW_EnemyLifeBar (UserInterface|GetUserWidgetObject (Variables|Default|GetWidget))))
    (Variables|/Game/_MagoOscar/Widgets/W_EnemyLifeBar.W_EnemyLifeBar_C|SetHealth _asw_enemy_life_bar _output_get)
    (if (<= _output_get 0.0)
      (CallFunction|Death)
      (Utilities|FlowControl|Delay 3.0)
      (Actor|DestroyActor)
      (else
        (CallFunction|RecibeDamage)
        (Utilities|FlowControl|Delay 0.7)
        (Components|Animation|SetAnimationMode (Variables|Character|GetMesh) "AnimationBlueprint" true)
        (Variables|Default|SetIsDamaged false)
        (Variables|/Script/Engine.CharacterMovementComponent|SetMaxWalkSpeed (Variables|Character|GetCharacterMovement) 3e+02)
        (CallFunction|FollowPlayer (Game|Player|GetPlayerPawn 0))))))

(event Custom|MoveAround
  (if (not (Variables|Default|GetIsDamaged))
    (if (not (Variables|Default|GetIsDying))
      (bind _randomlocation (Class|NavigationSystemV1|GetRandomLocationinNavigableRadius (Transformation|GetActorLocation) 1e+03 0 0))
      (Utilities|FlowControl|Delay 3.7)
      (AI|AIMoveTo self _randomlocation 0 5.0 false
        (:OnSuccess
          (CallFunction|MoveAround))))))

(event Game|Damage|EventAnyDamage
  (params (Damage :type Float%20%28single-precision%29) (DamageType :type Damage%20Type%20Object%20Reference) (InstigatedBy :type Controller%20Object%20Reference) (DamageCauser :type Actor%20Object%20Reference))
  (Development|PrintString (Utilities|GetDisplayName DamageCauser))
  (if (!= DamageCauser self)
    (CallFunction|TakeDamage Damage)))

(event EventBeginPlay
  (CallFunction|MoveAround))

(fn ConstructionScript)

(fn Death
  (Variables|Default|SetIsDying true)
  (Components|Animation|PlayAnimation (Variables|Character|GetMesh) "/Game/_MagoOscar/Animation/Animation/GoblinAnim/Death.Death" false)
  (Variables|/Script/Engine.CharacterMovementComponent|SetMaxWalkSpeed (Variables|Character|GetCharacterMovement) 0.0))

(fn Attack
  (Variables|Default|SetIsAttacking true)
  (Components|Animation|PlayAnimation (Variables|Character|GetMesh) "/Game/_MagoOscar/Animation/Animation/GoblinAnim/New/Sword_And_Shield_Slash.Sword_And_Shield_Slash" false))

(fn RecibeDamage
  (Variables|Default|SetIsDamaged true)
  (Components|Animation|PlayAnimation (Variables|Character|GetMesh) "/Game/_MagoOscar/Animation/Animation/GoblinAnim/Impact.Impact" false)
  (Variables|/Script/Engine.CharacterMovementComponent|SetMaxWalkSpeed (Variables|Character|GetCharacterMovement) 0.0))