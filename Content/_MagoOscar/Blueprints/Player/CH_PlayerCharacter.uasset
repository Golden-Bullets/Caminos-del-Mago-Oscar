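; Player character Blueprint that handles jumping, movement and camera look through Enhanced Input actions.
; Move input drives movement along the actor's right and forward vectors, scaled by MoveSpeed as an input multiplier.
; Look input feeds controller yaw and pitch scaled by Sensibility, and prints the scaled pitch value as debug text.
; The construction script is empty.
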(event Input|EnhancedActionEvents|EnhancedInputActionIA_Jump
  (params (ActionValue :type Boolean) (ElapsedSeconds :type Float%20%28double-precision%29) (TriggeredSeconds :type Float%20%28double-precision%29) (InputAction :type Input%20Action%20Object%20Reference :default "/Game/_MagoOscar/Input/IA_Jump.IA_Jump"))
  (Character|Jump))

(event Input|EnhancedActionEvents|EnhancedInputActionIA_Move
  (params (ActionValue :type Vector%202D%20Structure) (ElapsedSeconds :type Float%20%28double-precision%29) (TriggeredSeconds :type Float%20%28double-precision%29) (InputAction :type Input%20Action%20Object%20Reference :default "/Game/_MagoOscar/Input/IA_Move.IA_Move"))
  (bind _movespeed (Variables|Default|GetMoveSpeed))
  ;[1 1 1] Moverse
  (Pawn|Input|AddMovementInput (Transformation|GetActorRightVector) (* (.x ActionValue) _movespeed) false)
  (Pawn|Input|AddMovementInput (Transformation|GetActorForwardVector) (* (.y ActionValue) _movespeed) false))

(event Input|EnhancedActionEvents|EnhancedInputActionIA_Look
  (params (ActionValue :type Vector%202D%20Structure) (ElapsedSeconds :type Float%20%28double-precision%29) (TriggeredSeconds :type Float%20%28double-precision%29) (InputAction :type Input%20Action%20Object%20Reference :default "/Game/_MagoOscar/Input/IA_Look.IA_Look"))
  (bind _sensibility (Variables|Default|GetSensibility))
  (bind _returnvalue (* (.y ActionValue) _sensibility))
  ;[1 1 1] Camara
  ;;[1 1 1] El Yaw es para mirar a los lados
  (Pawn|Input|AddControllerYawInput (* (.x ActionValue) _sensibility))
  ;;[1 1 1] El pitch es para mirar arriba y abajo
  (Pawn|Input|AddControllerPitchInput _returnvalue)
  (Development|PrintText (Utilities|Text|ToText(Float) _returnvalue "HalfToEven")))

(fn ConstructionScript)