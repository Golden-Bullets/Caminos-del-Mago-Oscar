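; BP_Puzzle03 is an interactable combination puzzle that rewards a green gem when solved.
; Its Check event compares three key values against a hard-coded code while CanBeSolved is true.
; On a match it spawns BP_GreenGem at its own transform and clears CanBeSolved, so the reward spawns only once.
; The file shows neither what sets the keys nor what calls Check.
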(event Custom|Check
  (if (Variables|Default|GetCanBeSolved)
    (if (== (Variables|Default|GetKey01) 6)
      (if (== (Variables|Default|GetKey02) 8)
        (if (== (Variables|Default|GetKey03) 1)
          (Game|SpawnActorfromClass "/Game/_MagoOscar/Blueprints/Interactables/BP_GreenGem.BP_GreenGem_C" (Transformation|GetActorTransform) "Undefined" "MultiplyWithRoot" 0 0)
          (Variables|Default|SetCanBeSolved false))))))

(fn ConstructionScript)